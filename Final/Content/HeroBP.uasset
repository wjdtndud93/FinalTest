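; HeroBP is the player character, moved along fixed world axes, turned by a yaw input, and armed with a gun.
; On BeginPlay it spawns a GunBP on the mesh's GunSocket, and the trigger input starts and stops its firing.
; Death disables input, spawns an emitter, hides the character and restarts the level after a short delay.
; Mouse-cursor marker logic remains in the graph but never runs.
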(event `InputAxis|MoveForward`
  (params (AxisValue :type "Float (single-precision)"))
  (`self.AddMovementInput` (10.0 0.0 0.0) AxisValue))

(event `InputAxis|MoveRight`
  (params (AxisValue :type "Float (single-precision)"))
  (`self.AddMovementInput` (0.0 10.0 0.0) AxisValue))

(event `InputAxis|Turn`
  (params (AxisValue :type "Float (single-precision)"))
  (`self.K2_AddActorLocalRotation` (`KismetMathLibrary.MakeRotator` 0.0 0.0 (* AxisValue 3.0))))

(event `self.ReceiveBeginPlay`
  (`self.GetGun`))

(event `InputAction|BulleetTrigger`
  (params (Key :type "Key Structure" :default "AnyKey"))
  (bind _gun (`self.Gun`))
  (:`Pressed`
    (`/Game/Gun/GunBP.FireStart` _gun))
  (:`Released`
    (`/Game/Gun/GunBP.FireStop` _gun)))

(event `InputAction|LeftMouseClicked`
  (params (Key :type "Key Structure" :default "AnyKey")))

(event `Death`
  (`self.DisableInput` (`GameplayStatics.GetPlayerController` 0))
  (`GameplayStatics.SpawnEmitterAtLocation` null (`self.K2_GetActorLocation`))
  (`SceneComponent.SetVisibility` (`self.CapsuleComponent`) false true)
  (`KismetSystemLibrary.Delay` 2.0)
  (`KismetSystemLibrary.ExecuteConsoleCommand` "RestartLevel"))

(fn `GetGun`
  (bind _returnvalue (`|SpawnActorFromClass` "/Game/Gun/GunBP.GunBP_C" (`SceneComponent.K2_GetComponentToWorld` (`self.Mesh`)) "Undefined" "OverrideRootScale"))
  (bind _output_get (set `self.Gun` _returnvalue))
  (`self.K2_AttachToComponent` _output_get (`self.Mesh`) "GunSocket" "SnapToTarget" "SnapToTarget" "KeepWorld" true))

(fn `UserConstructionScript`)