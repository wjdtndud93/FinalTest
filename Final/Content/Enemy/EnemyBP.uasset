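; EnemyBP is an enemy actor that takes damage and kills the hero on contact.
; It sets HP at BeginPlay, and the DecreaseHP event subtracts damage and destroys the actor once HP runs out.
; A hit on its Box component casts the other actor to HeroBP and calls Death on it.
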(event `self.ReceiveBeginPlay`
  (set `self.HP` 100.0))

(event `/Game/Interface/DamageInterface.DecreaseHP`
  (params (Amount :type "Float (single-precision)"))
  (bind _output_get (set `self.HP` (- (`self.HP`) Amount)))
  (if (<= _output_get 0.0)
    (`self.K2_DestroyActor`)))

(event `self.Box.OnComponentHit`
  (params (HitComponent :type "PrimitiveComponent Object Reference") (OtherActor :type "Actor Object Reference") (OtherComp :type "PrimitiveComponent Object Reference") (NormalImpulse :type "Vector Structure") (Hit :type "HitResult Structure (by ref)"))
  (bind _ashero_bp (cast `/Game/HeroBP` OtherActor))
  (`/Game/HeroBP.Death` _ashero_bp))

(fn `UserConstructionScript`)